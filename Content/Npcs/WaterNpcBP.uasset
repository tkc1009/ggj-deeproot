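; Water NPC actor that rises steadily along world Z while the game is in play.
; On BeginPlay it caches GameMode_BP, then each tick moves itself upward by its move speed, frame time and the game mode's speed, without sweeping.
; The same tick sets the uniform scale of its WaterNpcPlane, doubling the size while bonus mode is active.
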(event EventBeginPlay
  (bind _asgame_mode_bp (Utilities|Casting|CastToGameMode_BP (Game|GetGameMode)))
  (Variables|Default|SetgameMode _asgame_mode_bp))

(event Collision|EventActorBeginOverlap
  (params (OtherActor :type Actor%20Object%20Reference)))

(event EventTick
  (params (DeltaSeconds :type Float%20%28single-precision%29))
  (bind _gamemode (Variables|Default|GetgameMode))
  (bind _waternpcplane (Variables|Default|GetWaterNpcPlane))
  (Variables|Default|SetdeltaTime DeltaSeconds)
  (if (Default|IsinGame _gamemode)
    (Utilities|FlowControl|Sequence
      (:then_0
        (Transformation|SetActorLocation (+ (Transformation|GetActorLocation) (* (Math|Vector|MakeVector 0.0 0.0 1.0) (* (Variables|Default|GetMOVE_SPEED_UP) (Variables|Default|GetdeltaTime) (Variables|/Game/System/GameMode_BP.GameMode_BP_C|GetgameSpeed (Variables|Default|GetgameMode))))) false false))
      (:then_1
        (if (Utilities|IsValid _waternpcplane)
          (Transformation|SetWorldScale3D _waternpcplane (Math|Conversions|ToVector(Float) (Math|Float|SelectFloat 0.09 0.045 (Variables|/Game/System/GameMode_BP.GameMode_BP_C|GetisBonusMode _gamemode)))))))))

(fn ConstructionScript)