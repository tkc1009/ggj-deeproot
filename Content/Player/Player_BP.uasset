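; Player Blueprint for a steering game: left/right input turns a clamped angle that tilts the mesh and drives sideways movement, scaled by game speed.
; A chain of sphere meshes spawned at BeginPlay follows along Y, each link easing at capped speed toward a blend of its neighbors.
; Overlaps report to GameMode_BP: water is collected, rocks are smashed in turbo mode, and anything else ends the game.
; Also handles pause and development-only fullscreen toggle.
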(event OnComponentBeginOverlap(PlayerMeshCollision)
  (params (OverlappedComponent :type Primitive%20Component%20Object%20Reference) (OtherActor :type Actor%20Object%20Reference) (OtherComp :type Primitive%20Component%20Object%20Reference) (OtherBodyIndex :type Integer) (bFromSweep :type Boolean) (SweepResult :type Hit%20Result%20Structure%20%28by%20ref%29))
  (bind _returnvalue (Transformation|GetActorLocation OtherActor))
  (bind _gamemode (Variables|Default|GetGameMode))
  (Utilities|FlowControl|Sequence
    (:then_0
      (Development|PrintString (Utilities|String|Append "OVERLAP " (Utilities|GetDisplayName OtherActor)) false))
    (:then_1
      (bind _aswater_npc_bp (Utilities|Casting|CastToWaterNpcBP OtherActor)
        (:then
          (Default|NotifyGetWater _gamemode)
          (Utilities|FlowControl|Sequence
            (:then_0
              (Niagara|SpawnSystematLocation "/Game/Effects/ExplosionWater.ExplosionWater" _returnvalue))
            (:then_1
              (Actor|DestroyActor _aswater_npc_bp)
              (Audio|PlaySound2D "/Game/Audio/Waterdrops/waterDropRandom_Cue.waterDropRandom_Cue" 1.0 1.0 0.0 0 0))))
        (:CastFailed
          (Utilities|Casting|CastToRockNpc_BP OtherActor
            (:then
              (if (Variables|/Game/System/GameMode_BP.GameMode_BP_C|GetisTurboMode _gamemode)
                (Utilities|FlowControl|Sequence
                  (:then_0
                    (Niagara|SpawnSystematLocation "/Game/Effects/Explosion.Explosion" _returnvalue "0, 0, 0" (Math|Conversions|ToVector(Float) (Math|Float|MakeLiteralFloat 1.0))))
                  (:then_1
                    (Actor|DestroyActor OtherActor)
                    (Default|NotifyDestroyRock _gamemode)
                    (Audio|PlaySound2D "/Game/Audio/Rocksmash/rockSmashRandom_Cue.rockSmashRandom_Cue" 1.0 1.0 0.0 0 0)))
                (else
                  (Default|GameOver _gamemode))))
            (:CastFailed
              (Default|GameOver _gamemode))))))))

(event EventBeginPlay
  (bind _returnvalue (Transformation|GetActorLocation))
  (bind (_x _y _z) (Math|Vector|BreakVector _returnvalue))
  (Utilities|FlowControl|Sequence
    (:then_0
      (bind _asgame_mode_bp (Utilities|Casting|CastToGameMode_BP (Game|GetGameMode)))
      (Variables|Default|SetGameMode _asgame_mode_bp))
    (:then_1
      (for _index (range 0 (- (Variables|Default|GetCHAIN_MESH_COUNT) 1))
        (bind _returnvalue_2 (Game|AddComponentbyClass "/Script/Engine.StaticMeshComponent" true (Math|Conversions|ToTransform(Vector) (Math|Vector|MakeVector (+ _x 1.8) _y (+ (* _index (/ (Variables|Default|GetCHAIN_DISTANCE_TOTAL) (Math|Conversions|ToFloat(Integer) (Variables|Default|GetCHAIN_MESH_COUNT)))) (Variables|Default|GetCHAIN_INITIAL_OFFSET) _z)))))
        (Collision|SetCollisionEnabled _returnvalue_2 "NoCollision")
        (Components|StaticMesh|SetStaticMesh _returnvalue_2 "/Engine/BasicShapes/Sphere.Sphere")
        (Rendering|Material|SetMaterial _returnvalue_2 0 "/Game/Player/M_PlayerMatChain.M_PlayerMatChain")
        (Transformation|SetWorldScale3D _returnvalue_2 (Math|Conversions|ToVector(Float) (Variables|Default|GetCHAIN_SCALE)))
        (Utilities|Array|Add (Variables|Default|GetchainArray) _returnvalue_2)))))

(event EventTick
  (params (DeltaSeconds :type Float%20%28single-precision%29))
  (bind _playermeshplane (Variables|Default|GetPlayerMeshPlane))
  (bind _max_angle (Variables|Default|GetMAX_ANGLE))
  (bind _returnvalue (Transformation|GetWorldRotation _playermeshplane))
  (bind (_roll _pitch _yaw) (Math|Rotator|BreakRotator _returnvalue))
  (Variables|Default|SetdeltaTime DeltaSeconds)
  (if (Default|IsinGame (Variables|Default|GetGameMode))
    (Utilities|FlowControl|Sequence
      (:then_0
        (Variables|Default|SetinputLRValue (+ (* (Math|Conversions|ToFloat(Boolean) (Variables|Default|GetisPressingLeft)) -1.0) (Math|Conversions|ToFloat(Boolean) (Variables|Default|GetisPressingRight))))
        (Variables|Default|SetplayerAngle (Math|Float|Clamp(Float) (+ (Variables|Default|GetplayerAngle) (* (Variables|Default|GetinputLRValue) (Variables|Default|GetTURN_RATE) (Variables|Default|GetdeltaTime))) (* _max_angle -1.0) _max_angle))
        (Transformation|SetActorLocation (+ (Transformation|GetActorLocation) (* "0,1.000000, 0" (* (Math|Trig|Sin(Degrees) (Variables|Default|GetplayerAngle)) (Variables|Default|GetLR_MOVE_SPEED) (Variables|Default|GetdeltaTime) (Variables|/Game/System/GameMode_BP.GameMode_BP_C|GetgameSpeed (Variables|Default|GetGameMode))))) false false))
      (:then_1
        (Transformation|SetRelativeRotation _playermeshplane (Math|Rotator|MakeRotator _roll (* (Variables|Default|GetplayerAngle) -1.0) _yaw) false false))
      (:then_2
        (for (_ _array_index) (Variables|Default|GetchainArray)
          (CallFunction|UpdateChainMeshbyIndex _array_index))))))

(event Input|ActionEvents|InputActionLeft
  (params (Key :type Key%20Structure))
  (:Pressed
    (Variables|Default|SetisPressingLeft true))
  (:Released
    (Variables|Default|SetisPressingLeft false)))

(event Input|ActionEvents|InputActionRight
  (params (Key :type Key%20Structure))
  (:Pressed
    (Variables|Default|SetisPressingRight true))
  (:Released
    (Variables|Default|SetisPressingRight false)))

(event Input|ActionEvents|InputActionPause
  (params (Key :type Key%20Structure))
  (:Pressed
    (if (Default|IsinGame (Variables|Default|GetGameMode))
      (Game|SetGamePaused (not (Game|IsGamePaused))))))

(event Input|KeyboardEvents|F10
  (params (Key :type Key%20Structure))
  (:Pressed
    (if (not (Class|KismetSystemLibrary|IsPackagedforDistribution))
      (Development|ExecuteConsoleCommand "MainFrame.ToggleFullscreen" 0))))

(fn ConstructionScript)

(fn UpdateChainMeshbyIndex
  (params (index :type Integer))
  (bind _returnvalue (- index 1))
  (bind _chainarray (Variables|Default|GetchainArray))
  (bind _output (Utilities|Array|Get(acopy) _chainarray index))
  (bind _returnvalue_2 (Transformation|GetWorldLocation _output))
  (bind (_x _y _z) (Math|Vector|BreakVector _returnvalue_2))
  (Utilities|FlowControl|Sequence ; calc goal y
    (:then_0
      (LocalVariables|SetcurrentY _y))
    (:then_1
      (if (< _returnvalue 0)
        (LocalVariables|SetprevIndexY (+ (* (.Y (Math|Vector|BreakVector (Transformation|GetActorLocation))) 1.03) (* (Math|Trig|Sin(Degrees) (Variables|Default|GetplayerAngle)) -1.5))) ; PLAYER POS, adjust by angle
        (else
          (LocalVariables|SetprevIndexY (.Y (Math|Vector|BreakVector (Transformation|GetWorldLocation (Utilities|Array|Get(acopy) (Variables|Default|GetchainArray) _returnvalue))))))))
    (:then_2
      (LocalVariables|SetnextIndexY (.Y (Math|Vector|BreakVector (Transformation|GetWorldLocation (Utilities|Array|Get(acopy) (Variables|Default|GetchainArray) (Math|Integer|Clamp(Integer) (+ index 1) 0 (- (Variables|Default|GetCHAIN_MESH_COUNT) 1))))))))
    (:then_3
      (LocalVariables|SetgoalY (Math|Float|Lerp (LocalVariables|GetprevIndexY) (LocalVariables|GetnextIndexY) 0.35)))
    (:then_4
      (Utilities|FlowControl|Sequence ; update y
        (:then_0
          (if (< (LocalVariables|GetgoalY) (LocalVariables|GetcurrentY))
            (LocalVariables|SetnewY (Math|Float|Max(Float) (- (LocalVariables|GetcurrentY) (* (Variables|Default|GetdeltaTime) (Variables|Default|GetCHAIN_MOVE_SPEED))) (LocalVariables|GetgoalY)))
            (else
              (LocalVariables|SetnewY (Math|Float|Min(Float) (LocalVariables|GetgoalY) (+ (LocalVariables|GetcurrentY) (* (Variables|Default|GetdeltaTime) (Variables|Default|GetCHAIN_MOVE_SPEED))))))))
        (:then_1
          (Transformation|SetWorldLocation _output (Math|Vector|MakeVector _x (LocalVariables|GetnewY) _z) false false))))))