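; Game mode for an arcade survival game that runs the flow from title screen through play to game over and level reload.
; While playing, Tick raises difficulty over time to quicken randomized rock and water spawns and computes score from time and pickups.
; Collected water fills a gauge that triggers a draining turbo mode, followed by a brief dry mode.
; These states drive a material parameter collection, and turbo crossfades the music.
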(event EventBeginPlay
  (Utilities|FlowControl|Sequence
    (:then_0
      (Utilities|FlowControl|Sequence
        (:then_0
          (bind _asplayer_controller_bp (Utilities|Casting|CastToPlayerController_BP (Game|GetPlayerController 0))
            (:then
              (Variables|Default|SetPlayerController _asplayer_controller_bp))
            (:CastFailed
              (Development|PrintText "ERROR: WRONG PLAYER CONTROLLER"))))
        (:then_1
          (bind _outactors (Actor|GetAllActorsOfClass "/Game/Player/PlayerCamera_BP.PlayerCamera_BP_C"))
          (for _array_element _outactors
            (Game|Player|SetViewTargetwithBlend (Variables|Default|GetPlayerController) _array_element 0.0 "VTBlend_Linear" 0.0 false)))
        (:then_2
          (bind _returnvalue (UserInterface|CreateWidget "/Game/UI/Title_UMG.Title_UMG_C" (Variables|Default|GetPlayerController)))
          (bind _output_get (Variables|Default|SettitleUmg _returnvalue))
          (UserInterface|Viewport|AddtoViewport _output_get 0))
        (:then_3
          (Input|SetInputModeGameandUI (Variables|Default|GetPlayerController) (Variables|Default|GettitleUmg) "DoNotLock" false)
          (Variables|/Script/Engine.PlayerController|SetbShowMouseCursor (Variables|Default|GetPlayerController) true)
          (Default|FocusonStartButton _output_get))
        (:then_4
          (Development|ExecuteConsoleCommand "r.OneFrameThreadLag 0" 0) ; reduces input latency
        )
        (:then_5
          (bind _returnvalue_2 (Audio|CreateSound2D "/Game/Audio/combinedMusic_Cue.combinedMusic_Cue" 1.0 1.0 0.0 0))
          (bind _output_get_2 (Variables|Default|Setbgm_component _returnvalue_2))
          (Audio|Components|Audio|Play _output_get_2 0.0))))
    (:then_1
      (if (and (not (Class|KismetSystemLibrary|IsPackagedforDistribution)) (Variables|Default|GetDEBUG_isSkipTitle)) ; DEBUG
        (CallFunction|StartGame)))))

(event EventTick
  (params (DeltaSeconds :type Float%20%28single-precision%29))
  (bind _default_game_speed (Variables|Default|GetDEFAULT_GAME_SPEED))
  (Variables|Default|SetdeltaTime DeltaSeconds)
  (Utilities|FlowControl|Sequence
    (:then_0
      (if (CallFunction|IsinGame)
        (Utilities|FlowControl|Sequence
          (:then_0
            (bind _output_get (Variables|Default|SettotalTime (+ (Variables|Default|GettotalTime) (Variables|Default|GetdeltaTime))))
            (Rendering|Material|SetScalarParameterValue "/Game/Materials/MatCollection_Custom.MatCollection_Custom" "TotalTime" _output_get :!class /Script/Engine.KismetMaterialLibrary))
          (:then_1
            (Variables|Default|Setdifficulty (+ (Math|Float|Floor (/ (Variables|Default|GettotalTime) 3.0)) 1)))
          (:then_2
            (Variables|Default|SetnextEnemySpawnTimer (- (Variables|Default|GetnextEnemySpawnTimer) (Variables|Default|GetdeltaTime)))
            (if (<= (Variables|Default|GetnextEnemySpawnTimer) 0.0)
              (Game|SpawnActorfromClass "/Game/Npcs/RockNpc_BP.RockNpc_BP_C" (Math|Conversions|ToTransform(Vector) (Math|Vector|MakeVector -6e+01 (* (Math|Random|RandomFloatinRange -1.0 1.0) 5e+01) -5e+01)) "AlwaysSpawn" self 0)
              (Variables|Default|SetnextEnemySpawnTimer (* (Math|Float|MapRangeClamped (Math|Conversions|ToFloat(Integer) (Variables|Default|Getdifficulty)) 1.0 1e+01 1.65 0.27) (Math|Random|RandomFloatinRange 0.43 1.2)))))
          (:then_3
            (Variables|Default|SetnextWaterSpawnTimer (- (Variables|Default|GetnextWaterSpawnTimer) (Variables|Default|GetdeltaTime)))
            (if (<= (Variables|Default|GetnextWaterSpawnTimer) 0.0)
              (Game|SpawnActorfromClass "/Game/Npcs/WaterNpcBP.WaterNpcBP_C" (Math|Conversions|ToTransform(Vector) (Math|Vector|MakeVector -6e+01 (* (Math|Random|RandomFloatinRange -1.0 1.0) 49.0) -5e+01)) "AlwaysSpawn" self 0)
              (Variables|Default|SetnextWaterSpawnTimer (+ (Math|Float|MapRangeClamped (Math|Conversions|ToFloat(Integer) (Variables|Default|Getdifficulty)) 1.0 1e+01 1.5 0.7) (* (Math|Random|RandomFloatinRange -1.0 1.0) 0.25)))))
          (:then_4
            (if (Variables|Default|GetisTurboMode)
              (Variables|Default|SetwaterGaugeRatio (Math|Float|Clamp(Float) (- (Variables|Default|GetwaterGaugeRatio) (* (Variables|Default|GetdeltaTime) (Variables|Default|GetTURBO_DEPLETION_RATE)))))
              (if (== (Variables|Default|GetwaterGaugeRatio) 0.0)
                (Variables|Default|SetisTurboMode false)
                (Variables|Default|SetdryModeTimer 2.0))))
          (:then_5
            (Rendering|Material|SetScalarParameterValue "/Game/Materials/MatCollection_Custom.MatCollection_Custom" "IsTurboMode" (Math|Conversions|ToFloat(Boolean) (Variables|Default|GetisTurboMode)) :!class /Script/Engine.KismetMaterialLibrary)
            (bind _output_get_2 (Variables|Default|SetdryModeTimer (- (Variables|Default|GetdryModeTimer) (Variables|Default|GetdeltaTime))))
            (Rendering|Material|SetScalarParameterValue "/Game/Materials/MatCollection_Custom.MatCollection_Custom" "IsDryMode" (Math|Conversions|ToFloat(Boolean) (> _output_get_2 0.0)) :!class /Script/Engine.KismetMaterialLibrary)
            (bind _output_get_3 (Variables|Default|SetisBonusMode (>= (Variables|Default|GetScore) 30000)))
            (Rendering|Material|SetScalarParameterValue "/Game/Materials/MatCollection_Custom.MatCollection_Custom" "IsBonusMode" (Math|Conversions|ToFloat(Boolean) _output_get_3) :!class /Script/Engine.KismetMaterialLibrary))
          (:then_6
            (Variables|Default|SetScore (+ (* (Math|Float|Floor (/ (Variables|Default|GettotalTime) 2.5)) 100) (* (Variables|Default|GetwaterGetCount) 300) (* (Variables|Default|GetrocksDestroyedCount) 500) 0)))
          (:then_7
            (Utilities|FlowControl|Sequence
              (:then_0
                (if (Variables|Default|GetisTurboMode)
                  (Variables|Default|SetgameSpeed (+ _default_game_speed 0.0))
                  (else
                    (Variables|Default|SetgameSpeed _default_game_speed))))
              (:then_1
                (Rendering|Material|SetScalarParameterValue "/Game/Materials/MatCollection_Custom.MatCollection_Custom" "GameSpeed" (Variables|Default|GetgameSpeed) :!class /Script/Engine.KismetMaterialLibrary))))
          (:then_8
            (Utilities|FlowControl|Sequence
              (:then_0
                (Variables|Default|SetturboCrossFadeRatio (Math|Float|Clamp(Float) (+ (Variables|Default|GetturboCrossFadeRatio) (* (Math|Float|SelectFloat 1e+01 -4.0 (Variables|Default|GetisTurboMode)) (Variables|Default|GetdeltaTime) 1.0)))))
              (:then_1
                (Audio|Parameter|SetFloatParameter (Variables|Default|Getbgm_component) "TurboCrossFade" (Variables|Default|GetturboCrossFadeRatio) :!class /Script/Engine.AudioComponent)))))))))

(fn ConstructionScript)

(fn StartGame
  (bind _playercontroller (Variables|Default|GetPlayerController))
  (Utilities|FlowControl|Sequence
    (:then_0
      (Widget|RemovefromParent (Variables|Default|GettitleUmg))
      (Variables|Default|SetisGameStarted true)
      (Input|SetInputModeGameOnly _playercontroller)
      (Variables|/Script/Engine.PlayerController|SetbShowMouseCursor _playercontroller false))
    (:then_1
      (Rendering|Material|SetScalarParameterValue "/Game/Materials/MatCollection_Custom.MatCollection_Custom" "PlayerMovementSpeedDown" 1.0 :!class /Script/Engine.KismetMaterialLibrary)
      (bind _returnvalue (UserInterface|CreateWidget "/Game/UI/HUD_UMG.HUD_UMG_C" (Variables|Default|GetPlayerController)))
      (Variables|Default|SethudUMG _returnvalue)
      (UserInterface|Viewport|AddtoViewport _returnvalue 0))
    (:then_2
      (Audio|PlaySound2D "/Game/Audio/Start_button_Cue.Start_button_Cue" 1.0 1.0 0.0 0 0))))

(fn GameOver
  (Utilities|FlowControl|Sequence
    (:then_0
      (Variables|Default|SetisGameOver true)
      (bind _returnvalue (UserInterface|CreateWidget "/Game/UI/Gameover_UMG.Gameover_UMG_C" (Variables|Default|GetPlayerController)))
      (bind _output_get (Variables|Default|SetgameoverUmg _returnvalue))
      (UserInterface|Viewport|AddtoViewport _returnvalue 0)
      (Input|SetInputModeGameandUI (Variables|Default|GetPlayerController) _returnvalue "DoNotLock" false)
      (Variables|/Script/Engine.PlayerController|SetbShowMouseCursor (Variables|Default|GetPlayerController) true)
      (Rendering|Material|SetScalarParameterValue "/Game/Materials/MatCollection_Custom.MatCollection_Custom" "PlayerMovementSpeedDown" 0.0 :!class /Script/Engine.KismetMaterialLibrary)
      (Default|FocusonButton _output_get))
    (:then_1
      (Audio|Components|Audio|Stop (Variables|Default|Getbgm_component))
      (Audio|PlaySound2D "/Game/Audio/GameOver_stinger_Cue.GameOver_stinger_Cue" 1.0 1.0 0.0 0 0))
    (:then_2
      (Development|PrintString (Utilities|String|Append "game over. totalTime: " (Utilities|String|ToString(Float) (Variables|Default|GettotalTime)) " , difficulty: " (Utilities|String|ToString(Integer) (Variables|Default|Getdifficulty)) " , water gotten: " (Utilities|String|ToString(Integer) (Variables|Default|GetwaterGetCount)) " , rocks destroyed: " (Utilities|String|ToString(Integer) (Variables|Default|GetrocksDestroyedCount)) " , gameSpeed: " (Utilities|String|ToString(Float) (Variables|Default|GetgameSpeed))) false))))

(fn ReturntoTitle
  (Utilities|FlowControl|Sequence
    (:then_0
      (Development|PrintString "Return to title!" false))
    (:then_1
      (bind _returnvalue (Game|GetCurrentLevelName true))
      (Game|OpenLevel(byName) (Utilities|String|StringToName _returnvalue)))))

(fn IsinGame
  (return (and (Variables|Default|GetisGameStarted) (not (Variables|Default|GetisGameOver)))))

(fn NotifyGetWater
  (Variables|Default|SetwaterGetCount (+ (Variables|Default|GetwaterGetCount) 1))
  (if (Variables|Default|GetisTurboMode)
    (Variables|Default|SetwaterGaugeRatio (Math|Float|Clamp(Float) (+ (Variables|Default|GetwaterGaugeRatio) (Variables|Default|GetWATER_RECOVERY_TURBO))))
    (else
      (Variables|Default|SetwaterGaugeRatio (Math|Float|Clamp(Float) (+ (Variables|Default|GetwaterGaugeRatio) (Variables|Default|GetWATER_RECOVERY_NORMAL))))
      (if (>= (Variables|Default|GetwaterGaugeRatio) 1.0)
        (Variables|Default|SetisTurboMode true)))))

(fn NotifyDestroyRock
  (Variables|Default|SetrocksDestroyedCount (+ (Variables|Default|GetrocksDestroyedCount) 1)))